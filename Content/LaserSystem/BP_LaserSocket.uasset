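; BP_LaserSocket is a socket actor that turns an empty laser spawn into an active laser emitter.
; When a BP_EmptyLaserSpawn overlaps its sphere while unfilled, it notifies FPC via ActorIsDestroyed and destroys that actor.
; It then spawns a BP_LaserSpawn with a purple laser color at the static mesh's transform and marks the socket filled, so it triggers only once.
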(event OnComponentBeginOverlap(Sphere)
  (params (OverlappedComponent :type Primitive%20Component%20Object%20Reference) (OtherActor :type Actor%20Object%20Reference) (OtherComp :type Primitive%20Component%20Object%20Reference) (OtherBodyIndex :type Integer) (bFromSweep :type Boolean) (SweepResult :type Hit%20Result%20Structure%20%28by%20ref%29))
  (bind _staticmesh (Variables|Default|GetStaticMesh))
  (bind _returnvalue (Transformation|GetWorldTransform _staticmesh))
  (if (not (Variables|Default|GetSocketFilled))
    (bind _asbp_empty_laser_spawn (Utilities|Casting|CastToBP_EmptyLaserSpawn OtherActor))
    (Default|ActorIsDestroyed (Variables|Default|GetFPC))
    (Actor|DestroyActor _asbp_empty_laser_spawn)
    (Game|SpawnActorfromClass "/Game/LaserSystem/BP_LaserSpawn.BP_LaserSpawn_C" (Math|Transform|MakeTransform (.location _returnvalue) (.rotation _returnvalue) "1.000000,1.000000,1.000000") "Undefined" "MultiplyWithRoot" 0 "(R=0.803686,G=0.000000,B=1.000000,A=1.000000)" 0 0)
    (Variables|Default|SetSocketFilled true)))

(event EventBeginPlay)

(event Collision|EventActorBeginOverlap
  (params (OtherActor :type Actor%20Object%20Reference)))

(event EventTick
  (params (DeltaSeconds :type Float%20%28single-precision%29)))

(fn ConstructionScript)