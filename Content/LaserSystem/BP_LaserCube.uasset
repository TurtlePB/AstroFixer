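; BP_LaserCube is an interactable cube in the laser system that re-emits an incoming laser.
; LaserBounce spawns an attached BP_Laser along its arrow, passing on color and an updated ID and registering it with the spawn reference.
; A negative hit response powers it down and clears attached lasers.
; Focus toggles an outline via custom depth; interacting flips InteractToggle, whose OnRep only prints debug placeholders.
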(event Custom|Interact
  (Variables|Default|SetInteractToggle (not (Variables|Default|GetInteractToggle))))

(event EventInterfaceToggleFocus
  (params (Focus :type Boolean))
  (Rendering|SetRenderCustomDepth (Variables|Default|GetSM_Parent) Focus))

(event EventInterfaceInteract
  (CallFunction|Interact))

(fn ConstructionScript
  (|CallParentFunction))

(fn OnRepInteractToggle
  (if (Variables|Default|GetInteractToggle)
    ;[1 1 1] Remove and show witched for rotatino
    (Development|PrintString "Bitch")
    (else
      (Development|PrintString "noBitch"))))

(fn InterfaceGetInteractionWidget
  (return (Variables|Default|GetWidget)))

(fn LaserBounce
  (params (P-LaserHit :type BP%20Laser%20Object%20Reference) (P-HitResponse :type Boolean) (P-HitInformation :type Hit%20Result%20Structure))
  (Utilities|IsValid P-LaserHit
    (:Is%20Valid
      (Variables|Default|SetSpawnReference (Variables|/Game/LaserSystem/BP_LaserParent.BP_LaserParent_C|GetSpawnReference P-LaserHit))
      (bind _output_get (Variables|Default|SetActive P-HitResponse))
      (if _output_get
        (CallFunction|Activate/Deactivate "/Game/LaserSystem/SFX/SW_PowerOn.SW_PowerOn")
        (bind _returnvalue (Game|SpawnActorfromClass "/Game/LaserSystem/BP_Laser.BP_Laser_C" (Math|Transform|MakeTransform (Transformation|GetWorldLocation (Variables|Default|GetArrow)) (Math|Rotator|MakeRotfromZ (Math|Vector|GetForwardVector (Variables|Default|GetArrow))) "1.000000,1.000000,1.000000") "Undefined" "MultiplyWithRoot" 0 (Default|UpdateID P-LaserHit "C") (Variables|/Game/LaserSystem/BP_LaserParent.BP_LaserParent_C|GetLaserColor P-LaserHit) (Variables|Default|GetSpawnReference) 0))
        (Transformation|AttachComponentToComponent _returnvalue (Variables|Default|GetSM_Parent) "None" "KeepWorld" "KeepWorld" "KeepRelative" false)
        (Utilities|Array|Add (Variables|Default|GetLasersAttached) _returnvalue)
        (Utilities|Array|Add (Variables|/Game/LaserSystem/BP_LaserSpawn.BP_LaserSpawn_C|GetChildLaser (Variables|Default|GetSpawnReference)) _returnvalue)
        (return _returnvalue)
        (else
          (CallFunction|Activate/Deactivate "/Game/LaserSystem/SFX/SW_PowerDown.SW_PowerDown")
          (CallFunction|ClearAllLasersAttached))))))