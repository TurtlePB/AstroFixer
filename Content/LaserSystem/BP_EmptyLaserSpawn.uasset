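; BP_EmptyLaserSpawn is an interactable actor in the laser system, apparently a placeholder for a laser spawn point.
; It implements interaction interface calls that supply its Widget and switch custom depth rendering on its static mesh when focus changes.
; Interacting flips the InteractToggle variable, whose RepNotify only checks the value and has no effect yet, so no laser is spawned here.
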(event Custom|Interact
  (Variables|Default|SetinteractToggle (not (Variables|Default|GetinteractToggle))))

(event EventInterfaceInteract
  (CallFunction|Interact))

(event EventInterfaceToggleFocus
  (params (Focus :type Boolean))
  (Rendering|SetRenderCustomDepth (Variables|Default|GetStaticMesh) Focus))

(fn ConstructionScript)

(fn OnRepInteractToggle
  (if (Variables|Default|GetInteractToggle)
    _))

(fn InterfaceGetInteractionWidget
  (return (Variables|Default|GetWidget)))