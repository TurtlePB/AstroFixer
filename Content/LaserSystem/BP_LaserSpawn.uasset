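; BP_LaserSpawn is a laser emitter that spawns and tracks the BP_Laser beams of its chain.
; On BeginPlay it spawns the first laser at its Arrow, passing its display name as ID, its color and a self-reference.
; RemoveFollowingLasers walks ChildLaser backwards, calls CancelTargetHit on lasers whose ID contains the given laser's ID, flagging the exact match, and drops those returning true.
; Substring matching on IDs identifies downstream lasers without explicit links.
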(event EventBeginPlay
  (bind _self self)
  (Variables|Default|SetSpawnReference _self)
  (Variables|Default|SetID (Utilities|GetDisplayName _self))
  (bind _returnvalue (Game|SpawnActorfromClass "/Game/LaserSystem/BP_Laser.BP_Laser_C" (Math|Transform|MakeTransform (Transformation|GetWorldLocation (Variables|Default|GetArrow)) (Transformation|GetActorRotation) "1.000000,1.000000,1.000000") "Undefined" "MultiplyWithRoot" 0 (Variables|Default|GetID) (Variables|Default|GetLaserColor) (Variables|Default|GetSpawnReference) 0))
  (Utilities|Array|Add (Variables|Default|GetChildLaser) _returnvalue))

(fn ConstructionScript
  (|CallParentFunction))

(fn RemoveFollowingLasers
  (params (LaserReference :type BP%20Laser%20Object%20Reference))
  (LocalVariables|SetL-ID_Removed (Variables|/Game/LaserSystem/BP_Laser.BP_Laser_C|GetLaser_ID LaserReference))
  (bind _arrayelement (Utilities|Array|ReverseforEachLoop (Variables|Default|GetChildLaser))
    (:LoopBody
      (Utilities|IsValid _arrayelement
        (:Is%20Valid
          (if (Utilities|String|Contains (Variables|/Game/LaserSystem/BP_Laser.BP_Laser_C|GetLaser_ID _arrayelement) (LocalVariables|GetL-ID_Removed))
            (bind _removefromarray (Default|CancelTargetHit _arrayelement (Utilities|Enum|Equal(Enum) (Variables|/Game/LaserSystem/BP_Laser.BP_Laser_C|GetLaser_ID _arrayelement) (LocalVariables|GetL-ID_Removed))))
            (if _removefromarray
              (Utilities|Array|RemoveItem (Variables|Default|GetChildLaser) _arrayelement))))))))