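; Interactable reflector that bounces lasers by spawning a new BP_Laser at the impact point.
; LaserBounce rotates the child from hit data (its double normal mirror cancels out), copies color, extends the ID and registers it with itself and the spawn reference.
; A negative response destroys attached lasers whose IDs lack the incoming ID.
; Focus toggles custom depth, interaction flips a flag, and leaving the box releases a character holding a reflect wall.
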(event OnComponentEndOverlap(Box)
  (params (OverlappedComponent :type Primitive%20Component%20Object%20Reference) (OtherActor :type Actor%20Object%20Reference) (OtherComp :type Primitive%20Component%20Object%20Reference) (OtherBodyIndex :type Integer))
  (bind _asbp_first_person_character (Utilities|Casting|CastToBP_FirstPersonCharacter OtherActor))
  (if (Variables|/Game/FirstPerson/Blueprints/BP_FirstPersonCharacter.BP_FirstPersonCharacter_C|GetIsReflectWall _asbp_first_person_character)
    (Variables|/Game/FirstPerson/Blueprints/BP_FirstPersonCharacter.BP_FirstPersonCharacter_C|SetIsHolding _asbp_first_person_character false)
    (Variables|/Game/FirstPerson/Blueprints/BP_FirstPersonCharacter.BP_FirstPersonCharacter_C|SetIsReflectWall _asbp_first_person_character false)))

(event Custom|Interact
  (Variables|Default|SetInteractToggle (not (Variables|Default|GetInteractToggle))))

(event EventInterfaceInteract
  (CallFunction|Interact))

(event EventInterfaceToggleFocus
  (params (Focus :type Boolean))
  (Rendering|SetRenderCustomDepth (Variables|Default|GetSM_Parent) Focus))

(fn ConstructionScript
  (|CallParentFunction))

(fn ClearAttachedLasers
  (params (P-ID_Clear :type String))
  (bind _arrayelement (Utilities|Array|ReverseforEachLoop (Variables|Default|GetLasersAttached))
    (:LoopBody
      (Utilities|IsValid _arrayelement
        (:Is%20Valid
          (if (not (Utilities|String|Contains (Variables|/Game/LaserSystem/BP_Laser.BP_Laser_C|GetLaser_ID _arrayelement) P-ID_Clear))
            (Actor|DestroyActor _arrayelement)
            (Utilities|Array|RemoveItem (Variables|Default|GetLasersAttached) _arrayelement)))))))

(fn CalculateRotation
  (params (P-ImpactPoint :type Vector) (P-TraceStart :type Vector) (P-ImpactNormal :type Vector))
  (return (Math|Rotator|MakeRotfromZ (Math|Vector|MirrorVectorbyNormal (Math|Vector|MirrorVectorbyNormal (* P-ImpactPoint P-TraceStart) P-ImpactNormal) P-ImpactNormal))))

(fn OnRepInteractToggle
  (if (Variables|Default|GetInteractToggle)
    _))

(fn InterfaceGetInteractionWidget
  (return (Variables|Default|GetWidget)))

(fn LaserBounce
  (params (P-LaserHit :type BP%20Laser%20Object%20Reference) (P-HitResponse :type Boolean) (P-HitInformation :type Hit%20Result%20Structure))
  (bind (_bblockinghit _binitialoverlap _time _distance _location _impactpoint _normal _impactnormal _physmat _hitactor _hitcomponent _hitbonename _bonename _hititem _elementindex _faceindex _tracestart) (Collision|BreakHitResult P-HitInformation))
  (if P-HitResponse
    (bind _returnvalue (Game|SpawnActorfromClass "/Game/LaserSystem/BP_Laser.BP_Laser_C" (Math|Transform|MakeTransform _impactpoint (CallFunction|CalculateRotation _impactpoint _tracestart _impactnormal) "1.000000,1.000000,1.000000") "Undefined" "MultiplyWithRoot" 0 (Default|UpdateID P-LaserHit "B") (Variables|/Game/LaserSystem/BP_LaserParent.BP_LaserParent_C|GetLaserColor P-LaserHit) (Variables|/Game/LaserSystem/BP_LaserParent.BP_LaserParent_C|GetSpawnReference P-LaserHit) 0))
    (Utilities|Array|Add (Variables|Default|GetLasersAttached) _returnvalue)
    (Utilities|Array|Add (Variables|/Game/LaserSystem/BP_LaserSpawn.BP_LaserSpawn_C|GetChildLaser (Variables|/Game/LaserSystem/BP_LaserParent.BP_LaserParent_C|GetSpawnReference P-LaserHit)) _returnvalue)
    (return _returnvalue)
    (else
      (CallFunction|ClearAttachedLasers (Variables|/Game/LaserSystem/BP_Laser.BP_Laser_C|GetLaser_ID P-LaserHit)))))