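; BP_LaserTarget2 is a laser-system target that opens a linked wall while a laser activates it.
; LaserBounce stores the hit response as Active, then GotHitByLaser hides LinkedWall's mesh, disables its collision and hides ReflektorWall2, or restores all three when inactive.
; It tints a dynamic material with the laser color or gray, then immediately replaces it with a green or default solid material.
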(event EventBeginPlay)

(fn ConstructionScript
  (|CallParentFunction))

(fn GotHitbyLaser
  (params (ColorLaser :type Linear%20Color%20Structure))
  (bind _linkedwall (Variables|Default|GetLinkedWall))
  (bind _sm_parent (Variables|Default|GetSM_Parent))
  (bind _reflektorwall2 (Variables|Default|GetReflektorWall2))
  (bind _wall (Variables|/Game/LaserSystem/BP_LaserWall.BP_LaserWall_C|GetWall _linkedwall))
  (bind _returnvalue (Rendering|Material|CreateDynamicMaterialInstance (Variables|Default|GetSM_Parent) 0 "/Game/LevelPrototyping/Materials/M_Solid.M_Solid" "None" :!class /Script/Engine.PrimitiveComponent))
  (Rendering|Material|SetVectorParameterValue _returnvalue " Base Color" (Math|Color|SelectColor ColorLaser "(R=0.213542,G=0.213542,B=0.213542,A=1.000000)" (Variables|Default|GetActive)) :!class /Script/Engine.MaterialInstanceDynamic)
  (if (Variables|Default|GetActive)
    (Rendering|Material|SetMaterial _sm_parent 0 "/Game/LevelPrototyping/Materials/MI_Solid_Green.MI_Solid_Green")
    (Utilities|IsValid _linkedwall
      (:Is%20Valid
        (Rendering|SetVisibility _wall false true)
        (Collision|SetCollisionEnabled _wall "NoCollision")
        (Rendering|SetActorHiddenInGame _reflektorwall2 true)))
    (else
      (Rendering|Material|SetMaterial _sm_parent 0 "/Game/LevelPrototyping/Materials/M_Solid.M_Solid")
      (Utilities|IsValid _linkedwall
        (:Is%20Valid
          (Rendering|SetVisibility _wall true true)
          (Collision|SetCollisionEnabled _wall "QueryAndPhysics")
          (Rendering|SetActorHiddenInGame _reflektorwall2 false))))))

(fn LaserBounce
  (params (P-LaserHit :type BP%20Laser%20Object%20Reference) (P-HitResponse :type Boolean) (P-HitInformation :type Hit%20Result%20Structure))
  (Variables|Default|SetActive P-HitResponse)
  (CallFunction|GotHitbyLaser (Variables|/Game/LaserSystem/BP_LaserParent.BP_LaserParent_C|GetLaserColor P-LaserHit))
  (return 0))